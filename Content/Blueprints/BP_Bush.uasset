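; BP_Bush is an actor that reacts when the third-person character overlaps it.
; On overlap it casts the other actor, prints a debug message and activates an explosion effect; other actors only get a "No player" message.
; A disconnected chain would push the player away from the bush with an impulse and destroy the bush after a delay, but it never runs.
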(event `self.ReceiveActorBeginOverlap`
  (params (OtherActor :type "Actor Object Reference"))
  (bind _asthird_person_character (cast `/Game/ThirdPersonBP/Blueprints/ThirdPersonCharacter` OtherActor)
    (:`then`
      (`KismetSystemLibrary.PrintString` "Hello" true true (struct :`R` 1.0 :`G` 0.072616 :`A` 1.0) 5.0)
      (`ActorComponent.Activate` (`self.FX_Explosion`) true))
    (:`CastFailed`
      (`KismetSystemLibrary.PrintString` "No player" true true (struct :`R` 1.0 :`G` 0.072616 :`A` 1.0) 5.0))))

(fn `UserConstructionScript`)